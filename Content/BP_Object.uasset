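; BP_Object is a game object that periodically jumps to random spots in the play area.
; On BeginPlay it caches BP_MyGameMode, then InitObject teleports it within fixed bounds and re-arms a timer on itself, with a delay that shrinks as PlayerLvl rises.
; A collect-and-respawn chain reporting to the game mode exists but is disconnected, so overlaps currently do nothing.
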(event `self.ReceiveBeginPlay`
  (bind _asbp_my_game_mode (cast `/Game/BP_MyGameMode` (`GameplayStatics.GetGameMode`)))
  (set `self.MyGamemode` _asbp_my_game_mode)
  (`self.InitObject`))

(event `self.ReceiveActorBeginOverlap`
  (params (OtherActor :type "Actor Object Reference")))

(fn `InitObject`
  (`self.K2_TeleportTo` (`KismetMathLibrary.MakeVector` (`KismetMathLibrary.RandomFloatInRange` -1800.0 1000.0) (`KismetMathLibrary.RandomFloatInRange` -1400.0 1400.0) 130.0))
  (`KismetSystemLibrary.K2_SetTimer` null "InitObject" (`KismetMathLibrary.Conv_IntToDouble` (- 6 (`/Game/BP_MyGameMode.PlayerLvl` (`self.MyGamemode`))))))

(fn `UserConstructionScript`)
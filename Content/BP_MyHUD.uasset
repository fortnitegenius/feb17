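; BP_MyHUD is a HUD Blueprint that draws points, time, a level label and a game-over screen with a retry prompt.
; DrawHUD renders text at fixed screen positions each frame, reading Points, Time and the GameOver flag through its Gamemode variable.
; BeginPlay casts to BP_MyGameMode but sets Gamemode to None, and the Level label has no value connected.
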(event `self.ReceiveBeginPlay`
  (cast `/Game/BP_MyGameMode` (`GameplayStatics.GetGameMode`))
  (set `self.Gamemode` null))

(event `self.ReceiveDrawHUD`
  (params (SizeX :type Integer) (SizeY :type Integer))
  (`self.DrawText` (`KismetStringLibrary.BuildString_Int` "Points" "" (`/Game/BP_MyGameMode.Points` (`self.Gamemode`))) (struct :`R` 0.162756 :`G` 0.031479 :`B` 0.581597 :`A` 1.0) 10.0 10.0 null 3.0)
  (`self.DrawText` (`KismetStringLibrary.BuildString_Int` "Time:" "" (`/Game/BP_MyGameMode.Time` (`self.Gamemode`))) (struct :`R` 1.0 :`G` 0.113526 :`B` 0.021225 :`A` 1.0) 300.0 10.0 null 3.0)
  (`self.DrawText` (`KismetStringLibrary.BuildString_Int` "Level:") (struct :`R` 0.019045 :`G` 0.307292 :`A` 1.0) 500.0 10.0 null 3.0)
  (if (`/Game/BP_MyGameMode.GameOver` (`self.Gamemode`))
    (`self.DrawText` "GAME OVER!! GIT GUD!!" (struct :`R` 0.425347 :`B` 0.002457 :`A` 1.0) 400.0 200.0 null 3.0)
    (`self.DrawText` "Press Enter to TRY AGAIN" (struct :`R` 0.425347 :`B` 0.002457 :`A` 1.0) 400.0 400.0 null 3.0)))

(fn `UserConstructionScript`)
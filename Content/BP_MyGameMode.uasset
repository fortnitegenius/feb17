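; Game mode that runs a timed collection game, tracking points, player level, time left and game-over state.
; The GameStart macro resets state on BeginPlay or GameRestart and starts a looping one-second Clock timer that counts down to game over.
; ObjectCollect awards level-scaled points, with time bonuses and capped level-ups on a modulo-five count check.
; ObjectCount adds zero, so that check passes on every pickup.
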(event `self.ReceiveBeginPlay`
  ;[0.06182 0.4729 0.8281 0.5] Uses GameStart Macro
  (`self.GameStart`))

(event `GameRestart`
  ;[0.06182 0.4729 0.8281 0.5] Uses GameStart Macro
  (`self.GameStart`))

(event `Clock`
  (bind _output_get (set `self.Time` (- (`self.Time`) 1)))
  (if (== _output_get 0)
    (set `self.GameOver` true)
    ;[0 0 0 0.5] .
    (`KismetSystemLibrary.K2_ClearTimer` null "Clock")))

(fn `ObjectCollect`
  (set `self.Points` (+ (`self.Points`) (* (`self.PlayerLvl`) 10)))
  (bind _output_get (set `self.ObjectCount` (+ (`self.ObjectCount`) 0)))
  (if (== (mod _output_get 5) 0)
    (set `self.Time` (+ (`self.Time`) 15))
    (set `self.PlayerLvl` (`KismetMathLibrary.Min` (+ (`self.PlayerLvl`) 1) 5))))

(fn `UserConstructionScript`)